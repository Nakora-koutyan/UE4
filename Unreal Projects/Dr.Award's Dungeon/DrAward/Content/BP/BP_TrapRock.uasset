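; BP_TrapRock is a trap actor that spawns a BP_Rock when play begins.
; Its construction script rotates HoleWallStart toward HoleWallEndLocation and adds a second static mesh at that location facing back, so the two hole walls always face each other.
; The spawn call has no transform wired in, as the Arrow component's world transform is left unconnected.
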(event `self.ReceiveBeginPlay`
  (`|SpawnActorFromClass` "/Game/BP/BP_Rock.BP_Rock_C" (struct) "Undefined" "OverrideRootScale" null null))

(fn `UserConstructionScript`
  (bind _holewallstart (`self.HoleWallStart`))
  (bind _holewallendlocation (`self.HoleWallEndLocation`))
  (bind _relativelocation (`SceneComponent.RelativeLocation` _holewallstart))
  (`SceneComponent.K2_SetRelativeRotation` _holewallstart (`KismetMathLibrary.FindLookAtRotation` _relativelocation _holewallendlocation) false false)
  (`AddComponent|NODE_AddStaticMeshComponent-0` :`RelativeTransform` (`KismetMathLibrary.MakeTransform` _holewallendlocation (`KismetMathLibrary.FindLookAtRotation` _holewallendlocation _relativelocation))))