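; BP_AwardGameMode is a game mode that respawns the player as a BP_Award whenever their pawn is destroyed.
; On BeginPlay it binds to player 0's pawn OnDestroyed event and prints a "Hello" debug string.
; The handler spawns a new BP_Award at a found player start, has player controller 0 possess it, then rebinds so the cycle repeats.
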(event `self.ReceiveBeginPlay`
  (`self.RespownEvent`))

(event `RespownEvent`
  (add `self.OnDestroyed` (`GameplayStatics.GetPlayerPawn` 0) (delegate `respawn_Award`))
  (`KismetSystemLibrary.PrintString` "Hello"))

(event `respawn_Award` :!signature `self.OnDestroyed`
  (params (DestroyedActor :type "Actor Object Reference"))
  (bind _returnvalue (`|SpawnActorFromClass` "/Game/BP/BP_Award.BP_Award_C" (`self.GetTransform` (`self.K2_FindPlayerStart` null)) "Undefined" "OverrideRootScale" null null))
  (`Controller.Possess` (`GameplayStatics.GetPlayerController` 0) _returnvalue)
  (`self.RespownEvent`))

(fn `UserConstructionScript`)